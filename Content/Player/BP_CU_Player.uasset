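; Player Blueprint for a dice game that lets the mouse pick up and drag dice and owns the score calculation widget.
; Left-click traces under the cursor for a BP_Dice and opens a Tick gate until release.
; While dragging, a camera-to-cursor ray intersected with a horizontal plane at pickup height positions the die mesh, zeroing its velocities.
; Separate events load starter dice from a data table and toggle score visibility.
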(event Custom|CreateStarterDice
  (bind _defaltdice (Variables|Default|GetDefaltDice))
  (bind _outrownames (DataTable|GetDataTableRowNames _defaltdice))
  (for _array_element _outrownames
    (bind _returnvalue (Utilities|GetDataTableRow _defaltdice _array_element)
      (:then
        (Utilities|Array|Add (Variables|Default|GetStarterDiceDataArray) _returnvalue)))))

(event Custom|HideScore
  (bind _calcscore_widget (Variables|Default|GetCalcScore_Widget))
  (Utilities|FlowControl|FlipFlop
    (:A
      (Widget|SetVisibility _calcscore_widget "Collapsed"))
    (:B
      (Widget|SetVisibility _calcscore_widget "Visible"))))

(event EventBeginPlay
  (Variables|/Script/Engine.PlayerController|SetbShowMouseCursor (Game|GetPlayerController 0) true)
  (bind _returnvalue (UserInterface|CreateWidget "/Game/Widgets/W_CalulateScore.W_CalulateScore_C"))
  (bind _output_get (Variables|Default|SetCalcScore_Widget _returnvalue))
  (UserInterface|Viewport|AddtoViewport _output_get 0))

(event EventTick
  (params (DeltaSeconds :type Float%20%28single-precision%29))
  (bind _returnvalue (Game|GetPlayerController 0))
  (bind _dicepickupzoffset (Variables|Default|GetDicePickUpZOffset))
  (bind _screenspaceoffset (Variables|Default|GetScreenSpaceOffset))
  (bind _hitactor (Variables|Default|GetHitActor))
  (bind _hitactor_2 (Variables|Default|GetHitActor))
  (bind (_worldlocation _worlddirection) (Game|Player|ConvertMouseLocationToWorldSpace _returnvalue))
  (bind _returnvalue_2 (Transformation|GetActorLocation _hitactor_2))
  (bind _ascu_player_controller (Utilities|Casting|CastToCU_PlayerController _returnvalue))
  (bind _dicemesh (Variables|/Game/Dice/BP_Dice.BP_Dice_C|GetDiceMesh _hitactor))
  (bind _returnvalue_3 (* _worldlocation _screenspaceoffset))
  (bind _returnvalue_4 (* _worlddirection 1e+04))
  (bind _cam (Variables|/Game/Player/CU_PlayerController.CU_PlayerController_C|GetCam _ascu_player_controller))
  (bind _returnvalue_5 (Transformation|GetActorLocation _cam))
  (bind _returnvalue_6 (+ _returnvalue_3 _returnvalue_4))
  (bind _intersection (Class|KismetMathLibrary|LinePlaneIntersectionOriginNormal _returnvalue_5 _returnvalue_6 (Math|Vector|MakeVector (.x _returnvalue_2) (.y _returnvalue_2) _dicepickupzoffset) "0.000000,0.000000,1.000000"))
  (Utilities|FlowControl|Gate true :!label _label
    (:Exit
      (Utilities|IsValid (Variables|Default|GetHitActor)
        (:Is%20Valid
          (Transformation|SetWorldLocation _dicemesh (Math|Vector|MakeVector (.x _intersection) (.y _intersection) (.z _intersection)) false true)
          (Class|PrimitiveComponent|SetAllPhysicsLinearVelocity _dicemesh "0, 0, 0" false)
          (Class|PrimitiveComponent|SetAllPhysicsAngularVelocityinDegrees _dicemesh (Math|Vector|MakeVector 0.0 0.0 0.0) false))
        (:Is%20Not%20Valid
          (goto _label Close))))))

(event Input|MouseEvents|LeftMouseButton
  (params (Key :type Key%20Structure :default "None"))
  (bind _returnvalue (Game|GetPlayerController 0))
  (bind _returnvalue_2 (Game|GetPlayerController 0))
  (bind _hitresult (Game|Player|GetHitResultUnderCursorbyChannel _returnvalue "TraceTypeQuery1" true))
  (bind (_worldlocation _worlddirection) (Game|Player|ConvertMouseLocationToWorldSpace _returnvalue_2))
  (bind (_bblockinghit _binitialoverlap _time _distance _location _impactpoint _normal _impactnormal _physmat _hitactor) (Collision|BreakHitResult _hitresult))
  (:Pressed
    (if _bblockinghit
      (bind _asbp_dice (Utilities|Casting|CastToBP_Dice _hitactor))
      (Utilities|IsValid _asbp_dice
        (:Is%20Valid
          (Variables|Default|SetHitActor _asbp_dice)
          (Default|OnDragStart (Variables|Default|GetHitActor))
          (Utilities|FlowControl|Gate true) ; enters at Open
        ))))
  (:Released
    (Utilities|IsValid (Variables|Default|GetHitActor)
      (:Is%20Valid
        (Default|OnDragEnd (Variables|Default|GetHitActor)))
      (:Is%20Not%20Valid
        _))
    (Variables|Default|SetHitActor 0)
    (Utilities|FlowControl|Gate true) ; enters at Close
  ))

(fn ConstructionScript)