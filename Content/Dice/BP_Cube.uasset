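; Dice cube actor whose sides each show a random number or operator symbol on text render components.
; On BeginPlay it fills SideData with random entries and writes them to the side texts; the level-based symbol argument is currently unused.
; GetUpSide finds the upward face by comparing each text's forward vector to world up with dot products, returning that side's data and printing its text every Tick.
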(event Custom|UpdateCube
  (for (_array_element _array_index) (Variables|Default|GetSideTextRenderArray)
    (Rendering|Components|TextRender|SetText _array_element (.operation (Utilities|Array|Get(acopy) (Variables|Default|GetSideData) _array_index)))))

(event Custom|RandomizeSides
  (CallFunction|SetSides (/ (Variables|Default|Getlevel) 5))
  (CallFunction|UpdateCube))

(event Custom|LockCubeRotOnClick)

(event EventBeginPlay
  (Variables|Default|SetSideTextRenderArray (Actor|GetComponentsByClass "/Script/Engine.TextRenderComponent"))
  (CallFunction|RandomizeSides)
  (CallFunction|UpdateCube))

(event EventTick
  (params (DeltaSeconds :type Float%20%28single-precision%29))
  (Development|PrintString (.ReturnValue (CallFunction|GetUpSide))))

(fn ConstructionScript)

(fn SetSides
  (params (SymbolLevel :type Integer))
  (LocalVariables|SetLOCAL_SymbolLevel SymbolLevel)
  (for (_ _array_index) (Variables|Default|GetSideData)
    (LocalVariables|SetLOCAL_SideArrayIndex _array_index)
    (bind _data (CallFunction|GetVaulue))
    (Utilities|Array|SetArrayElem (Variables|Default|GetSideData) (LocalVariables|GetLOCAL_SideArrayIndex) _data)))

(fn GetVaulue
  (params (SimbolLevel :type Integer))
  (bind _returnvalue (Math|Random|RandomIntegerinRange 0 6))
  (bind _output_get (LocalVariables|SetLOCAL_Symbol (Math|Random|RandomBool)))
  (if _output_get
    (bind _output_get_2 (Variables|Default|SetSymbolType (Utilities|Enum|ByteToEnumE_Symbols (Math|Conversions|ToByte(Integer) (Math|Random|RandomIntegerinRange 0 (- (|GetNumEnumEntries) 1))))))
    (return (Utilities|Struct|MakeDiceSide_Struct true 0 (|GenerictoText _output_get_2)))
    (else
      (return (Utilities|Struct|MakeDiceSide_Struct false _returnvalue (Utilities|Text|ToText(Integer) _returnvalue))))))

(fn GetUpSide
  (for (_array_element _array_index) (Variables|Default|GetSideTextRenderArray)
    (if (> (Math|Vector|DotProduct (Math|Vector|GetForwardVector _array_element) (Math|Vector|GetUpVector "0, 0, 0")) (LocalVariables|GetmostUp))
      (LocalVariables|SetmostUp (Math|Vector|DotProduct (Math|Vector|GetForwardVector _array_element) (Math|Vector|GetUpVector "0, 0, 0")))
      (LocalVariables|SetmostUpVector (Math|Vector|GetForwardVector _array_element))
      (LocalVariables|SetmostUpText _array_element)
      (LocalVariables|SetLocalArrayIndex _array_index)
      (else
        (LocalVariables|SetmostUp (LocalVariables|GetmostUp))
        (LocalVariables|SetmostUpVector (LocalVariables|GetmostUpVector))
        (LocalVariables|SetmostUpText (LocalVariables|GetmostUpText)))))
  (Development|PrintText (Variables|/Script/Engine.TextRenderComponent|GetText (LocalVariables|GetmostUpText)))
  (return (LocalVariables|GetmostUpVector) (Utilities|Array|Get(acopy) (Variables|Default|GetSideData) (LocalVariables|GetLocalArrayIndex)) ""))