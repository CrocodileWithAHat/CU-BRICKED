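; Draggable physics die whose six text faces each show a random number or symbol, with the side data stored in an array.
; Finds the upward face by comparing each text component's forward vector with world up.
; Drag start snaps to that face's preset rotation and disables physics and collision.
; Release restores both, then after a short delay locks rotation with a physics constraint, swapping materials to mark drag state.
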(event Custom|UpdateCube
  (for (_array_element _array_index) (Variables|Default|GetSideTextRenderArray)
    (Rendering|Components|TextRender|SetText _array_element (.operation (Utilities|Array|Get(acopy) (Variables|Default|GetSideData) _array_index)))))

(event Custom|RandomizeSides
  (CallFunction|SetSidesRandom (/ (Variables|Default|Getlevel) 5))
  (CallFunction|UpdateCube))

(event Custom|OnDragStart
  (bind _physicsconstraint (Variables|Default|GetPhysicsConstraint))
  (CallFunction|SnaptoTextDirection)
  (Class|PhysicsConstraintComponent|BreakConstraint _physicsconstraint)
  (Components|Activation|SetActive _physicsconstraint false false)
  (Physics|SetSimulatePhysics (Variables|Default|GetDiceMesh) false)
  (Collision|SetCollisionEnabled (Variables|Default|GetDiceMesh) "NoCollision")
  (Rendering|Material|SetMaterial (Variables|Default|GetDiceMesh) 0 "/AnimationSharing/AnimSharingGreen.AnimSharingGreen"))

(event Custom|readData
  (for _array_element (Variables|Default|GetSideData)
    (Development|PrintText (.Operation (Utilities|Struct|BreakDiceSide_Struct _array_element)))))

(event Custom|OnDragEnd
  (bind _dicemesh (Variables|Default|GetDiceMesh))
  (bind _physicsconstraint (Variables|Default|GetPhysicsConstraint))
  (bind _dicemesh_2 (Variables|Default|GetDiceMesh))
  (Physics|SetSimulatePhysics _dicemesh true)
  (Collision|SetCollisionEnabled _dicemesh "QueryAndPhysics")
  (Utilities|FlowControl|Delay 0.2)
  (Components|Activation|SetActive _physicsconstraint true false)
  (Class|PhysicsConstraintComponent|SetConstrainedComponents _physicsconstraint (Variables|Default|GetDiceMesh) "None" 0 "None")
  (Class|PhysicsConstraintComponent|SetAngularTwistLimit _physicsconstraint "ACM_Locked" 0.0)
  (Class|PhysicsConstraintComponent|SetAngularSwing1Limit _physicsconstraint "ACM_Locked" 0.0)
  (Class|PhysicsConstraintComponent|SetAngularSwing2Limit _physicsconstraint "ACM_Locked" 0.0)
  (Class|PrimitiveComponent|SetAllPhysicsAngularVelocityinDegrees _dicemesh_2 (Math|Vector|MakeVector 0.0 0.0 0.0) false)
  (Rendering|Material|SetMaterial _dicemesh_2 0 "/AnimationSharing/AnimSharingRed.AnimSharingRed"))

(event Custom|SnapToNearest90
  (bind _dicemesh (Variables|Default|GetDiceMesh))
  (bind _returnvalue (Transformation|GetWorldRotation _dicemesh))
  (Transformation|SetWorldRotation (Variables|Default|GetDiceMesh) (Math|Rotator|MakeRotator (Math|Conversions|ToFloat(Integer) (* (Math|Float|Round (/ (.roll _returnvalue) 9e+01)) 90)) (Math|Conversions|ToFloat(Integer) (* (Math|Float|Round (/ (.pitch _returnvalue) 9e+01)) 90)) (Math|Conversions|ToFloat(Integer) (* (Math|Float|Round (/ (.yaw _returnvalue) 9e+01)) 90))) false false))

(event Custom|SnapToTextDirection
  (bind _mostuptextcomponent (CallFunction|GetUpSide))
  (bind _returnvalue (Utilities|GetObjectName _mostuptextcomponent))
  (Variables|Default|SetSideRotIndex 0)
  (Development|PrintString _returnvalue)
  (switch string _returnvalue
    (:Top
      (Variables|Default|SetSideRotIndex 0))
    (:Right
      (Variables|Default|SetSideRotIndex 1))
    (:Front
      (Variables|Default|SetSideRotIndex 2))
    (:Back
      (Variables|Default|SetSideRotIndex 3))
    (:Bottom
      (Variables|Default|SetSideRotIndex 4))
    (:Left
      (Variables|Default|SetSideRotIndex 5)))
  (Transformation|SetWorldRotation (Variables|Default|GetDiceMesh) (Utilities|Array|Get(acopy) (Variables|Default|GetSideRots) (Variables|Default|GetSideRotIndex)) false false))

(event EventBeginPlay
  (Utilities|FlowControl|Sequence
    (:then_0
      (Class|PrimitiveComponent|SetMaxDepenetrationVelocity (Variables|Default|GetDiceMesh) "None" 0.0)
      (Class|PhysicsConstraintComponent|BreakConstraint (Variables|Default|GetPhysicsConstraint)))
    (:then_1
      (Variables|Default|SetSideTextRenderArray (Actor|GetComponentsByClass "/Script/Engine.TextRenderComponent")))))

(fn ConstructionScript)

(fn SetSidesRandom
  (params (SymbolLevel :type Integer))
  (LocalVariables|SetLOCAL_SymbolLevel SymbolLevel)
  (for (_ _array_index) (Variables|Default|GetSideData)
    (LocalVariables|SetLOCAL_SideArrayIndex _array_index)
    (bind _data (CallFunction|GetValuetoSetSide))
    (Utilities|Array|SetArrayElem (Variables|Default|GetSideData) (LocalVariables|GetLOCAL_SideArrayIndex) _data)))

(fn GetValuetoSetSide
  (bind _returnvalue (Math|Random|RandomIntegerinRange 0 6))
  (bind _output_get (LocalVariables|SetLOCAL_Symbol (Math|Random|RandomBool)))
  (if _output_get
    (return (Utilities|Struct|MakeDiceSide_Struct true 0 (|GenerictoText (Utilities|Enum|ByteToEnumE_Symbols (Math|Conversions|ToByte(Integer) (Math|Random|RandomIntegerinRange 0 (- (|GetNumEnumEntries) 1)))))))
    (else
      (return (Utilities|Struct|MakeDiceSide_Struct false _returnvalue (Utilities|Text|ToText(Integer) _returnvalue))))))

(fn GetUpSide
  (for (_array_element _array_index) (Variables|Default|GetSideTextRenderArray)
    (if (> (Math|Vector|DotProduct (Math|Vector|GetForwardVector _array_element) (Math|Vector|GetUpVector "0, 0, 0")) (LocalVariables|GetmostUp))
      (LocalVariables|SetmostUp (Math|Vector|DotProduct (Math|Vector|GetForwardVector _array_element) (Math|Vector|GetUpVector "0, 0, 0")))
      (LocalVariables|SetmostUpVector (Math|Vector|GetForwardVector _array_element))
      (LocalVariables|SetmostUpText _array_element)
      (LocalVariables|SetLocalArrayIndex _array_index)
      (else
        (LocalVariables|SetmostUp (LocalVariables|GetmostUp))
        (LocalVariables|SetmostUpVector (LocalVariables|GetmostUpVector))
        (LocalVariables|SetmostUpText (LocalVariables|GetmostUpText)))))
  (bind _output_get (Variables|Default|SetUpSideData (Utilities|Array|Get(acopy) (Variables|Default|GetSideData) (LocalVariables|GetLocalArrayIndex))))
  (return (LocalVariables|GetmostUpVector) _output_get (Utilities|String|ToString(Text) (Variables|/Script/Engine.TextRenderComponent|GetText (LocalVariables|GetmostUpText))) (LocalVariables|GetLocalArrayIndex) (LocalVariables|GetmostUpText)))

(fn UpdateSide
  (params (side :type Integer) (Data :type Dice%20Side%20Struct%20Structure))
  (Utilities|Array|SetArrayElem (Variables|Default|GetSideData) side Data))