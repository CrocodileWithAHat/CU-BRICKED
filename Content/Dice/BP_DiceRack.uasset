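; Dice rack actor that spawns a scaled grid of BP_RackSlot actors and scores the dice placed in them.
; CalulateScore reads each slot's up-face in row and column passes, folding values with symbol dice as operators (+, -, X, /, ^) into totals.
; CheckAllDiceUsed compares filled slots against the player's dice.
; UpdateSlots changes slot count, grows the grid and respawns, but ClearSlots is empty, its cleanup logic disconnected.
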(event EventBeginPlay
  (Variables|Default|SetStartPosition (Transformation|GetWorldLocation (Variables|Default|GetDefaultSceneRoot)))
  (CallFunction|SlotSpawner))

(event Collision|EventActorBeginOverlap
  (params (OtherActor :type Actor%20Object%20Reference)))

(event EventTick
  (params (DeltaSeconds :type Float%20%28single-precision%29)))

(fn ConstructionScript)

(fn SlotSpawner
  (bind _slotcounter (LocalVariables|GetSlotCounter))
  (bind _rackscaler (Variables|Default|GetrackScaler))
  (bind _slotcounter_2 (LocalVariables|GetSlotCounter))
  (bind _slotspacing (Variables|Default|GetSlotSpacing))
  (bind _startposition (Variables|Default|GetStartPosition))
  (for _index (range 0 (- (Variables|Default|GetSlotColumnCount) 1))
    (LocalVariables|SetLOCAL_ColumnIndex _index)
    (for _index_2 (range 0 (- (Variables|Default|GetSlotRowCount) 1))
      (LocalVariables|SetLOCAL_RowIndex _index_2)
      (if (< _slotcounter (Variables|Default|GetSlotCount))
        (bind _returnvalue (Game|SpawnActorfromClass "/Game/Dice/BP_RackSlot.BP_RackSlot_C" (Math|Transform|MakeTransform (Math|Vector|MakeVector (- (.x _startposition) (* (LocalVariables|GetLOCAL_RowIndex) (* (.x _slotspacing) _rackscaler))) (+ (.y _startposition) (* (LocalVariables|GetLOCAL_ColumnIndex) (* (.y _slotspacing) _rackscaler))) (.z _startposition)) (Transformation|GetWorldRotation (Variables|Default|GetDefaultSceneRoot)) (Math|Conversions|ToVector(Float) (* (Variables|Default|GetrackScaler) 1.0))) "AlwaysSpawn" "MultiplyWithRoot" 0 0))
        (bind _output_get (Variables|Default|SetLocationString (Utilities|String|Append "Row: " (Utilities|String|ToString(Integer) (LocalVariables|GetLOCAL_RowIndex)) "<br>Column: " (Utilities|String|ToString(Integer) (LocalVariables|GetLOCAL_ColumnIndex)) "<br>Slot Count: " (Utilities|String|ToString(Integer) _slotcounter))))
        (Default|SetLocationtext _returnvalue (Utilities|Text|ToText(String) _output_get))
        (Utilities|Array|SetArrayElem (Variables|Default|GetSlotArray) _slotcounter_2 _returnvalue true)
        (Math|Integer|IncrementInt _slotcounter_2)))))

(fn CalulateScore
  (Utilities|FlowControl|Sequence
    (:then_0
      ;[0 0.027 0.15 0.5] Calc Columns
      (for _index (range 0 (- (Variables|Default|GetSlotRowCount) 1))
        (LocalVariables|SetLOCAL_RowIndex _index)
        (for _index_2 (range 0 (- (Variables|Default|GetSlotColumnCount) 1))
          (LocalVariables|SetLOCAL_ColumnIndex _index_2)
          (if (>= (LocalVariables|GetLOCAL_slotIndex) (Variables|Default|GetSlotCount))
            (LocalVariables|SetLOCAL_TotalScore (+ (LocalVariables|GetLOCAL_TotalScore) (LocalVariables|GetLOCAL_ColumnScore)))
            (Variables|Default|SetSymbol "+")
            (LocalVariables|SetLOCAL_ColumnTotals (+ (LocalVariables|GetLOCAL_ColumnScore) (LocalVariables|GetLOCAL_ColumnTotals)))
            (LocalVariables|SetLOCAL_ColumnScore 0)
            (else
              (bind (_upsidedata _hascube) (Default|CheckSlot (Utilities|Array|Get(acopy) (Variables|Default|GetSlotArray) (LocalVariables|GetLOCAL_slotIndex))))
              (if _hascube
                (if (.Symbol (Utilities|Struct|BreakDiceSide_Struct _upsidedata))
                  (Variables|Default|SetSymbol (Utilities|String|ToString(Text) (.Operation (Utilities|Struct|BreakDiceSide_Struct _upsidedata))))
                  (Math|Integer|IncrementInt (LocalVariables|GetLOCAL_slotIndex))
                  (else
                    (bind _output (CallFunction|Calulate (Math|Conversions|ToFloat(Integer) (LocalVariables|GetLOCAL_ColumnScore)) (Math|Conversions|ToFloat(Integer) (.Value (Utilities|Struct|BreakDiceSide_Struct _upsidedata))) (Variables|Default|GetSymbol)))
                    (LocalVariables|SetLOCAL_ColumnScore (Math|Float|Truncate _output))
                    (Variables|Default|SetSymbol "+")
                    (Math|Integer|IncrementInt (LocalVariables|GetLOCAL_slotIndex))))
                (else
                  (Variables|Default|SetSymbol "+")
                  (Math|Integer|IncrementInt (LocalVariables|GetLOCAL_slotIndex)))))))
        (LocalVariables|SetLOCAL_TotalScore (+ (LocalVariables|GetLOCAL_TotalScore) (LocalVariables|GetLOCAL_ColumnScore)))
        (Variables|Default|SetSymbol "+")
        (LocalVariables|SetLOCAL_ColumnTotals (+ (LocalVariables|GetLOCAL_ColumnScore) (LocalVariables|GetLOCAL_ColumnTotals)))
        (LocalVariables|SetLOCAL_ColumnScore 0)))
    (:then_1
      ;[0.15 0.01711 0.01562 0.5] Calculate Rows
      (LocalVariables|SetLOCAL_slotIndex 0)
      (LocalVariables|SetLOCAL_RowIndex 0)
      (LocalVariables|SetLOCAL_ColumnIndex 0)
      (for _index_3 (range 0 (- (Variables|Default|GetSlotRowCount) 1))
        (LocalVariables|SetLOCAL_RowIndex _index_3)
        (for _index_4 (range 0 (- (Variables|Default|GetSlotColumnCount) 1))
          (LocalVariables|SetLOCAL_ColumnIndex _index_4)
          (if (>= (LocalVariables|GetLOCAL_slotIndex) (Variables|Default|GetSlotCount))
            (LocalVariables|SetLOCAL_TotalScore (+ (LocalVariables|GetLOCAL_TotalScore) (LocalVariables|GetLOCAL_RowScore)))
            (Variables|Default|SetSymbol "+")
            (LocalVariables|SetLOCAL_RowTotals (+ (LocalVariables|GetLOCAL_RowScore) (LocalVariables|GetLOCAL_RowTotals)))
            (LocalVariables|SetLOCAL_RowScore 0)
            (else
              (bind (_upsidedata_2 _hascube_2) (Default|CheckSlot (Utilities|Array|Get(acopy) (Variables|Default|GetSlotArray) (+ (* (LocalVariables|GetLOCAL_ColumnIndex) (Variables|Default|GetSlotRowCount)) (LocalVariables|GetLOCAL_RowIndex)))))
              (if _hascube_2
                (if (.Symbol (Utilities|Struct|BreakDiceSide_Struct _upsidedata_2))
                  (Variables|Default|SetSymbol (Utilities|String|ToString(Text) (.Operation (Utilities|Struct|BreakDiceSide_Struct _upsidedata_2))))
                  (Math|Integer|IncrementInt (LocalVariables|GetLOCAL_slotIndex))
                  (else
                    (bind _output_2 (CallFunction|Calulate (Math|Conversions|ToFloat(Integer) (LocalVariables|GetLOCAL_RowScore)) (Math|Conversions|ToFloat(Integer) (.Value (Utilities|Struct|BreakDiceSide_Struct _upsidedata_2))) (Variables|Default|GetSymbol)))
                    (LocalVariables|SetLOCAL_RowScore (Math|Float|Truncate _output_2))
                    (Variables|Default|SetSymbol "+")
                    (Math|Integer|IncrementInt (LocalVariables|GetLOCAL_slotIndex))))
                (else
                  (Variables|Default|SetSymbol "+")
                  (Math|Integer|IncrementInt (LocalVariables|GetLOCAL_slotIndex)))))))
        (LocalVariables|SetLOCAL_TotalScore (+ (LocalVariables|GetLOCAL_TotalScore) (LocalVariables|GetLOCAL_RowScore)))
        (Variables|Default|SetSymbol "+")
        (LocalVariables|SetLOCAL_RowTotals (+ (LocalVariables|GetLOCAL_RowScore) (LocalVariables|GetLOCAL_RowTotals)))
        (LocalVariables|SetLOCAL_RowScore 0))
      (return (LocalVariables|GetLOCAL_TotalScore) (LocalVariables|GetLOCAL_RowTotals) (LocalVariables|GetLOCAL_ColumnTotals)))))

(fn Calulate
  (params (StartingNumber :type Float%20%28double-precision%29) (Secondary%20Number :type Float%20%28double-precision%29) (Operation :type String))
  (LocalVariables|SetLOCAL_StartNum StartingNumber)
  (LocalVariables|SetLOCAL_SecNum Secondary%20Number)
  (switch string Operation
    (:Default
      _)
    (:+
      _)
    (:-
      (bind _out (CallFunction|Subtract (LocalVariables|GetLOCAL_StartNum) (LocalVariables|GetLOCAL_SecNum)))
      (return _out ""))
    (:x
      (if (> (LocalVariables|GetLOCAL_StartNum) 0.0)
        (bind _out_2 (CallFunction|Multiply (LocalVariables|GetLOCAL_StartNum) (LocalVariables|GetLOCAL_SecNum)))
        (return _out_2 "")
        (else
          (bind _out_3 (CallFunction|Multiply 1.0 (LocalVariables|GetLOCAL_SecNum)))
          (return _out_3 ""))))
    (:/
      (if (> (LocalVariables|GetLOCAL_StartNum) 0.0)
        (bind _out_4 (CallFunction|Divide (LocalVariables|GetLOCAL_StartNum) (LocalVariables|GetLOCAL_SecNum)))
        (return _out_4 "")
        (else
          (bind _out_5 (CallFunction|Divide 1.0 (LocalVariables|GetLOCAL_SecNum)))
          (return _out_5 ""))))
    (:^
      (if (> (LocalVariables|GetLOCAL_StartNum) 0.0)
        (bind _out_6 (CallFunction|Exponent (LocalVariables|GetLOCAL_StartNum) (LocalVariables|GetLOCAL_SecNum)))
        (return _out_6 "")
        (else
          (bind _out_7 (CallFunction|Exponent 1.0 (LocalVariables|GetLOCAL_SecNum)))
          (return _out_7 "")))))
  (bind _out_8 (CallFunction|Add (LocalVariables|GetLOCAL_StartNum) (LocalVariables|GetLOCAL_SecNum)))
  (return _out_8 ""))

(fn Add
  (params (First :type Float%20%28double-precision%29) (Second :type Float%20%28double-precision%29))
  (return (+ First Second)))

(fn Subtract
  (params (First :type Float%20%28double-precision%29) (Second :type Float%20%28double-precision%29))
  (return (- First Second)))

(fn Multiply
  (params (First :type Float%20%28double-precision%29) (Second :type Float%20%28double-precision%29))
  (return (* First Second)))

(fn Divide
  (params (First :type Float%20%28double-precision%29) (Second :type Float%20%28double-precision%29))
  (return (/ First Second)))

(fn Exponent
  (params (First :type Float%20%28double-precision%29) (Second :type Float%20%28double-precision%29))
  (return (Math|Float|Power First Second)))

(fn CheckAllDiceUsed
  (for _array_element (Variables|Default|GetSlotArray)
    (bind _hascube (Default|CheckSlot _array_element))
    (if _hascube
      (Math|Integer|IncrementInt (LocalVariables|GetLOCAL_DiceCount))))
  (bind _asbp_cu_player (Utilities|Casting|CastToBP_CU_Player (Game|GetPlayerCharacter 0)))
  (return (<= (Utilities|Array|Length (Variables|/Game/Player/BP_CU_Player.BP_CU_Player_C|GetDiceArray _asbp_cu_player)) (LocalVariables|GetLOCAL_DiceCount))))

(fn UpdateSlots
  (params (SlotsToAdd :type Integer) (SlotsToRemove :type Integer))
  (bind _slotrowcount (Variables|Default|GetSlotRowCount))
  (bind _slotcolumncount (Variables|Default|GetSlotColumnCount))
  (CallFunction|ClearSlots)
  (Variables|Default|SetSlotCount (+ (Variables|Default|GetSlotCount) SlotsToAdd))
  (bind _output_get (Variables|Default|SetSlotCount (- (Variables|Default|GetSlotCount) SlotsToRemove)))
  (if (< _output_get (* _slotrowcount _slotcolumncount))
    _
    (elif (> _slotrowcount _slotcolumncount)
      (Math|Integer|IncrementInt (Variables|Default|GetSlotColumnCount)
        (:%20%20
          _))
      (else
        (Math|Integer|IncrementInt (Variables|Default|GetSlotRowCount)
          (:%20%20
            _)))))
  (CallFunction|SlotSpawner))

(fn ClearSlots)

(fn GetSlotData
  (return (Variables|Default|GetSlotArray) (Variables|Default|GetSlotCount) (Variables|Default|GetSlotRowCount) (Variables|Default|GetSlotColumnCount) (Variables|Default|GetSlotSpacing) (Variables|Default|GetStartPosition) (Variables|Default|GetrackScaler)))

(fn SetSlotData
  (params (SlotArray :type Array%20of%20BP%20Rack%20Slot%20Object%20References) (SlotCount :type Integer) (SlotRowCount :type Integer) (SlotColumnCount :type Integer) (SlotSpacing :type Vector) (StartPosition :type Vector) (rackScaler :type Float%20%28double-precision%29))
  (Variables|Default|SetSlotArray SlotArray)
  (Variables|Default|SetSlotCount SlotCount)
  (Variables|Default|SetSlotRowCount SlotRowCount)
  (Variables|Default|SetSlotColumnCount SlotColumnCount)
  (Variables|Default|SetSlotSpacing SlotSpacing)
  (Variables|Default|SetStartPosition StartPosition)
  (Variables|Default|SetrackScaler rackScaler))