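; BP_RackSlot is a dice rack slot actor that reports whether a die sits in it and which side faces up.
; CheckSlot takes the first BP_Dice overlapping SlotCollision, updates HasDice and returns that die's UpSideData, or Empty when none is found.
; A SetLocationtext event writes a supplied value to the slot's TextRender label.
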(event Custom|SetLocationtext
  (params (Value :type Text%20%28by%20ref%29))
  (Rendering|Components|TextRender|SetText (Variables|Default|GetTextRender) Value))

(event EventBeginPlay)

(event Collision|EventActorBeginOverlap
  (params (OtherActor :type Actor%20Object%20Reference)))

(event EventTick
  (params (DeltaSeconds :type Float%20%28single-precision%29)))

(fn ConstructionScript)

(fn CheckSlot
  (bind _slotcollision (Variables|Default|GetSlotCollision))
  (bind _overlappingactors (Collision|GetOverlappingActors _slotcollision "/Game/Dice/BP_Dice.BP_Dice_C" :!class /Script/Engine.PrimitiveComponent))
  (bind _output (Utilities|Array|Get(acopy) _overlappingactors))
  (if (Utilities|Array|IsValidIndex _overlappingactors)
    (Utilities|IsValid _output
      (:Is%20Valid
        (bind _asbp_dice (Utilities|Casting|CastToBP_Dice _output)
          (:then
            (bind _output_get (Variables|Default|SetHasDice true))
            (return (Variables|/Game/Dice/BP_Dice.BP_Dice_C|GetUpSideData _asbp_dice) _output_get))
          (:CastFailed
            _)))
      (:Is%20Not%20Valid
        _)))
  (bind _output_get_2 (Variables|Default|SetHasDice false))
  (return (LocalVariables|GetEmpty) _output_get_2))