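; Dice spawner actor that launches the player's BP_Dice with random rotation, spin and an impulse along its arrow.
; When active, it spawns starter dice from the player's starter data in a delayed self-calling loop, filling the player's DiceArray.
; On a new level it teleports existing dice away, then relaunches them from the spawner at random intervals.
; It can also add a random starter die or rescale all dice.
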(event Custom|SpawnStarterDice
  (if (Variables|Default|Getactive)
    (bind _asbp_cu_player (Utilities|Casting|CastToBP_CU_Player (Game|GetPlayerCharacter 0)))
    (Default|CreateStarterDice _asbp_cu_player)
    (bind _output_get (Variables|Default|SetStarterDiceArray (Variables|/Game/Player/BP_CU_Player.BP_CU_Player_C|GetStarterDiceDataArray _asbp_cu_player)))
    (Variables|Default|SetDiceToSpawn (Utilities|Array|Length _output_get))
    (CallFunction|StarterSpawn)))

(event Custom|StarterSpawn
  (bind _returnvalue (Math|Random|RandomFloatinRange 0.0 9e+01))
  (bind _returnvalue_2 (Math|Random|RandomFloatinRange -1.2e+02 1.2e+02))
  (bind _defaultsceneroot (Variables|Default|GetDefaultSceneRoot))
  (bind _returnvalue_3 (Transformation|GetWorldTransform _defaultsceneroot))
  (bind _returnvalue_4 (Game|SpawnActorfromClass "/Game/Dice/BP_Dice.BP_Dice_C" (Math|Transform|MakeTransform (.location _returnvalue_3) (Math|Rotator|MakeRotator _returnvalue _returnvalue _returnvalue) (.scale _returnvalue_3)) "Undefined" "MultiplyWithRoot" 0 0))
  (Default|SetScale _returnvalue_4 (Variables|Default|GetdiceScaler))
  (Class|PrimitiveComponent|AddAngularImpulseinDegrees (Variables|/Game/Dice/BP_Dice.BP_Dice_C|GetDiceMesh _returnvalue_4) (Math|Vector|MakeVector _returnvalue_2 _returnvalue_2 _returnvalue_2) "None" true)
  (Physics|AddImpulse (Variables|/Game/Dice/BP_Dice.BP_Dice_C|GetDiceMesh _returnvalue_4) (* (Variables|Default|GetImpulseStrenght) (Math|Vector|GetForwardVector (Variables|Default|GetArrow))) "None" true)
  (Variables|/Game/Dice/BP_Dice.BP_Dice_C|SetSideData _returnvalue_4 (Utilities|Struct|BreakDiceSides_Struct (Utilities|Array|Get(acopy) (Variables|Default|GetStarterDiceArray) (Variables|Default|GetDiceCount))))
  (Default|UpdateCube _returnvalue_4)
  (bind _asbp_cu_player (Utilities|Casting|CastToBP_CU_Player (Game|GetPlayerCharacter 0)))
  (Utilities|Array|Add (Variables|/Game/Player/BP_CU_Player.BP_CU_Player_C|GetDiceArray _asbp_cu_player) _returnvalue_4)
  (Utilities|FlowControl|Delay (Math|Conversions|ToFloat(Integer) (Math|Random|RandomIntegerinRange (Variables|Default|GetStarterSpawnTimerMin) (Variables|Default|GetStarterSpawnTimerMax))))
  (bind _result (Math|Integer|IncrementInt (Variables|Default|GetDiceCount))
    (:%20%20
      (if (< _result (Variables|Default|GetDiceToSpawn))
        (CallFunction|StarterSpawn)
        (else
          (Variables|Default|SetDiceCount 0)
          (Variables|Default|SetDiceToSpawn 0))))))

(event Custom|NewLevel
  (if (Variables|Default|Getactive)
    (bind _asbp_cu_player (Utilities|Casting|CastToBP_CU_Player (Game|GetPlayerCharacter 0)))
    (Variables|Default|SetDiceToSpawn (Utilities|Array|Length (Variables|/Game/Player/BP_CU_Player.BP_CU_Player_C|GetDiceArray _asbp_cu_player)))
    (for _array_element (Variables|/Game/Player/BP_CU_Player.BP_CU_Player_C|GetDiceArray _asbp_cu_player)
      (Transformation|SetWorldLocation (Variables|/Game/Dice/BP_Dice.BP_Dice_C|GetDiceMesh _array_element) "5000.000000,50000.000000,0.000000" false true)
      (Utilities|FlowControl|Delay (Math|Random|RandomFloatinRange (Variables|Default|GetSpawnTimerMin) (Variables|Default|GetSpawnTimerMax)) :!label _label)
      (CallFunction|SpawnPlayerDiceArray)
      (bind _result (Math|Integer|IncrementInt (Variables|Default|GetDiceCount))
        (:%20%20
          (if (< _result (Variables|Default|GetDiceToSpawn))
            (goto _label)
            (else
              (Variables|Default|SetDiceCount 0)
              (Variables|Default|SetDiceToSpawn 0))))))))

(event Custom|changeDiceScale
  (params (diceScaler :type Float%20%28double-precision%29))
  (Variables|Default|SetdiceScaler diceScaler)
  (bind _asbp_cu_player (Utilities|Casting|CastToBP_CU_Player (Game|GetPlayerCharacter 0)))
  (for _array_element (Variables|/Game/Player/BP_CU_Player.BP_CU_Player_C|GetDiceArray _asbp_cu_player)
    (Default|SetScale _array_element (Variables|Default|GetdiceScaler))))

(event Custom|SpawnRadomDefaultDice
  (bind _returnvalue (Math|Random|RandomFloatinRange -1.2e+02 1.2e+02))
  (bind _returnvalue_2 (Math|Random|RandomFloatinRange 0.0 9e+01))
  (bind _starterdicearray (Variables|Default|GetStarterDiceArray))
  (bind _defaultsceneroot (Variables|Default|GetDefaultSceneRoot))
  (bind _returnvalue_3 (Transformation|GetWorldTransform _defaultsceneroot))
  (bind _returnvalue_4 (Game|SpawnActorfromClass "/Game/Dice/BP_Dice.BP_Dice_C" (Math|Transform|MakeTransform (.location _returnvalue_3) (Math|Rotator|MakeRotator _returnvalue_2 _returnvalue_2 _returnvalue_2) (.scale _returnvalue_3)) "Undefined" "MultiplyWithRoot" 0 0))
  (Default|SetScale _returnvalue_4 (Variables|Default|GetdiceScaler))
  (Class|PrimitiveComponent|AddAngularImpulseinDegrees (Variables|/Game/Dice/BP_Dice.BP_Dice_C|GetDiceMesh _returnvalue_4) (Math|Vector|MakeVector _returnvalue _returnvalue _returnvalue) "None" true)
  (Physics|AddImpulse (Variables|/Game/Dice/BP_Dice.BP_Dice_C|GetDiceMesh _returnvalue_4) (* (Variables|Default|GetImpulseStrenght) (Math|Vector|GetForwardVector (Variables|Default|GetArrow))) "None" true)
  (Variables|/Game/Dice/BP_Dice.BP_Dice_C|SetSideData _returnvalue_4 (Utilities|Struct|BreakDiceSides_Struct (Utilities|Array|Get(acopy) _starterdicearray (Math|Random|RandomInteger (Utilities|Array|Length _starterdicearray)))))
  (Default|UpdateCube _returnvalue_4)
  (bind _asbp_cu_player (Utilities|Casting|CastToBP_CU_Player (Game|GetPlayerCharacter 0)))
  (Utilities|Array|Add (Variables|/Game/Player/BP_CU_Player.BP_CU_Player_C|GetDiceArray _asbp_cu_player) _returnvalue_4))

(event EventBeginPlay)

(fn ConstructionScript)

(fn SpawnPlayerDiceArray
  (bind _returnvalue (Math|Random|RandomFloatinRange 0.0 9e+01))
  (bind _returnvalue_2 (Math|Random|RandomFloatinRange -1.2e+02 1.2e+02))
  (bind _defaultsceneroot (Variables|Default|GetDefaultSceneRoot))
  (bind _returnvalue_3 (Transformation|GetWorldTransform _defaultsceneroot))
  (bind _asbp_cu_player (Utilities|Casting|CastToBP_CU_Player (Game|GetPlayerCharacter 0)))
  (bind _output_get (LocalVariables|SetLOCAL_PlayerDiceArray (Variables|/Game/Player/BP_CU_Player.BP_CU_Player_C|GetDiceArray _asbp_cu_player)))
  (for (_array_element _array_index) _output_get
    (if (== _array_index (Variables|Default|GetDiceCount))
      (Default|ResetDrag _array_element)
      (Class|PrimitiveComponent|SetAllPhysicsAngularVelocityinDegrees (Variables|/Game/Dice/BP_Dice.BP_Dice_C|GetDiceMesh _array_element) (Math|Vector|MakeVector 0.0 0.0 0.0) false)
      (Class|PrimitiveComponent|SetAllPhysicsLinearVelocity (Variables|/Game/Dice/BP_Dice.BP_Dice_C|GetDiceMesh _array_element) "0, 0, 0" false)
      (Transformation|SetWorldTransform (Variables|/Game/Dice/BP_Dice.BP_Dice_C|GetDiceMesh _array_element) (Math|Transform|MakeTransform (.location _returnvalue_3) (Math|Rotator|MakeRotator _returnvalue _returnvalue _returnvalue) (.scale _returnvalue_3)) false true)
      (Default|SetScale _array_element (Variables|Default|GetdiceScaler))
      (Class|PrimitiveComponent|AddAngularImpulseinDegrees (Variables|/Game/Dice/BP_Dice.BP_Dice_C|GetDiceMesh _array_element) (Math|Vector|MakeVector _returnvalue_2 _returnvalue_2 _returnvalue_2) "None" true)
      (Physics|AddImpulse (Variables|/Game/Dice/BP_Dice.BP_Dice_C|GetDiceMesh _array_element) (* (Variables|Default|GetImpulseStrenght) (Math|Vector|GetForwardVector (Variables|Default|GetArrow))) "None" true)
      (Default|UpdateCube _array_element))))